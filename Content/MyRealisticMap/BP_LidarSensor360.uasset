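; Simulated 360-degree lidar sensor actor that combines a point cloud with four-direction camera and semantic segmentation captures.
; BeginPlay creates render targets and an empty dynamic point cloud, packs camera FOV, pitch and offsets into bytes, and flags fisheye from post-process materials.
; Tick launches an async scan using the four cameras; its callback appends semantic readbacks from the segmentation captures and stores the output.
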(event Custom|MyTestDelegate_Event
  (params (SensorOut360 :type Lidar%20Sensor%20Out%20360%20Structure))
  (bind (_deptharrayout360 _colorarrayoutf _colorarrayoutl _colorarrayoutb _colorarrayoutr) (Utilities|Struct|BreakLidarSensorOut360 SensorOut360))
  (bind _semanticarrayout (Class|SensorSimulatorBPLibrary|ReadSemantic (Variables|Default|GetSegF)))
  (Utilities|Array|AppendArray _colorarrayoutf _semanticarrayout)
  (bind _semanticarrayout_2 (Class|SensorSimulatorBPLibrary|ReadSemantic (Variables|Default|GetSegR)))
  (Utilities|Array|AppendArray _colorarrayoutr _semanticarrayout_2)
  (bind _semanticarrayout_3 (Class|SensorSimulatorBPLibrary|ReadSemantic (Variables|Default|GetSegB)))
  (Utilities|Array|AppendArray _colorarrayoutb _semanticarrayout_3)
  (bind _semanticarrayout_4 (Class|SensorSimulatorBPLibrary|ReadSemantic (Variables|Default|GetSegL)))
  (Utilities|Array|AppendArray _colorarrayoutl _semanticarrayout_4)
  (Variables|Default|SetLidarSensorOut360 SensorOut360))

(event Collision|EventActorBeginOverlap
  (params (OtherActor :type Actor%20Object%20Reference)))

(event EventTick
  (params (DeltaSeconds :type Float%20%28single-precision%29))
  (if (Variables|Default|GetIsInitialized)
    (if (Variables|Default|GetIsInitialized_RT)
      (Class|SensorSimulatorBPLibrary|LidarSensorAsyncScan360 (Variables|Default|GetLidarPointsArray) (Variables|Default|GetPC_Lidar) (Variables|Default|GetCameraF) (Variables|Default|GetCameraL) (Variables|Default|GetCameraB) (Variables|Default|GetCameraR) (delegate Custom|MyTestDelegate_Event) true -15.0 15.0 (Variables|Default|GetLidarChannels) 3.6e+02 (Variables|Default|GetLidarRes) (Variables|Default|GetLidarRange)))))

(event EventBeginPlay
  (bind _cameraf (Variables|Default|GetCameraF))
  (bind _camerab (Variables|Default|GetCameraB))
  (bind _cameral (Variables|Default|GetCameraL))
  (bind _pc_lidar (Variables|Default|GetPC_Lidar))
  (bind _camerar (Variables|Default|GetCameraR))
  (bind _camera_infos (Variables|Default|Getcamera_infos))
  (bind _array (Utilities|Array|MakeArray _cameraf _camerar _camerab _cameral))
  (Utilities|FlowControl|Sequence
    (:then_0
      (CallFunction|SensorSetRenderTarget _array)
      (CallFunction|SensorSetRenderTarget (Utilities|Array|MakeArray (Variables|Default|GetSegF) (Variables|Default|GetSegR) (Variables|Default|GetSegB) (Variables|Default|GetSegL)))
      (Variables|Default|SetIsInitialized_RT true))
    (:then_1
      (Class|LidarPointCloudComponent|SetPointCloud _pc_lidar (Class|LidarPointCloudBlueprintLibrary|CreatePointCloudEmpty))
      (Class|LidarPointCloud|SetOptimizedforDynamicData (Variables|/Script/LidarPointCloudRuntime.LidarPointCloudComponent|GetPointCloud _pc_lidar) true)
      (Variables|Default|SetIsInitialized true))
    (:then_2
      (Utilities|Array|Clear (Variables|Default|Getcamera_infos))
      (bind _bytes (Class|SensorSimulatorBPLibrary|InttoBytes (Math|Float|Truncate (Variables|/Script/Engine.SceneCaptureComponent2D|GetFOVAngle (Variables|Default|GetCameraF)))))
      (Utilities|Array|AppendArray _camera_infos _bytes)
      (for _array_element _array
        (bind _bytes_2 (Class|SensorSimulatorBPLibrary|InttoBytes (Math|Float|Truncate (.pitch (Variables|/Script/Engine.SceneComponent|GetRelativeRotation _array_element)))))
        (Utilities|Array|AppendArray (Variables|Default|Getcamera_y) _bytes_2)
        (bind _bytes_3 (Class|SensorSimulatorBPLibrary|InttoBytes (Math|Float|Truncate (.x (Variables|/Script/Engine.SceneComponent|GetRelativeLocation _array_element)))))
        (Utilities|Array|AppendArray (Variables|Default|Getcamera_loc_x) _bytes_3)
        (bind _bytes_4 (Class|SensorSimulatorBPLibrary|InttoBytes (Math|Float|Truncate (.y (Variables|/Script/Engine.SceneComponent|GetRelativeLocation _array_element)))))
        (Utilities|Array|AppendArray (Variables|Default|Getcamera_loc_y) _bytes_4)
        (bind _bytes_5 (Class|SensorSimulatorBPLibrary|InttoBytes (Math|Float|Truncate (.z (Variables|/Script/Engine.SceneComponent|GetRelativeLocation _array_element)))))
        (Utilities|Array|AppendArray (Variables|Default|Getcamera_loc_z) _bytes_5))
      (Utilities|Array|AppendArray _camera_infos (Variables|Default|Getcamera_y))
      (Utilities|Array|AppendArray _camera_infos (Variables|Default|Getcamera_loc_x))
      (Utilities|Array|AppendArray _camera_infos (Variables|Default|Getcamera_loc_y))
      (Utilities|Array|AppendArray _camera_infos (Variables|Default|Getcamera_loc_z)))
    (:then_3
      (Variables|Default|SetIsFisheye (> (Utilities|Array|Length (Utilities|Struct|BreakWeightedBlendables (Utilities|Struct|BreakPostProcessSettings (Variables|/Script/Engine.SceneCaptureComponent2D|GetPostProcessSettings (Variables|Default|GetCameraF))))) 0)))))

(fn ConstructionScript)

(fn SensorSetRenderTarget
  (params (scenecapture2dArray :type Array%20of%20Scene%20Capture%20Component%202D%20Object%20References))
  (for _array_element scenecapture2dArray
    (bind _returnvalue (Rendering|CreateRenderTarget2D (Variables|Default|GetCaptureImageWidth) (Variables|Default|GetCaptureImageHeight) "RTF_RGBA8"))
    (bind _output_get (Variables|Default|SetCameraRenderTarget _returnvalue))
    (Variables|/Script/Engine.SceneCaptureComponent2D|SetTextureTarget _array_element _output_get)))