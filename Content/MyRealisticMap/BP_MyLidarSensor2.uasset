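; Simulated lidar sensor actor that scans its surroundings into a depth map and a live point cloud.
; While triggered, Tick finds BP_PC and, if its CreatePC is set, launches an async scan, using ScanCompleted to prevent overlapping scans.
; The completion callback stores depths and pushes points to BP_PC's point cloud.
; Clicking the lidar mesh prints the depth map length; GetDepthmap holds only disconnected leftovers, including UDP sending.
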(event OnClicked(SM_lidar)
  (params (TouchedComponent :type Primitive%20Component%20Object%20Reference) (ButtonPressed :type Key%20Structure :default "None"))
  (Development|PrintString (Utilities|String|ToString(Integer) (Utilities|Array|Length (Variables|Default|GetDepthmap))) true false))

(event Custom|CustomEvent_1
  (params (StringOut :type String))
  (Variables|Default|SetDepthmap (stale EventTick _deptharrayout))
  (Class|LidarPointCloud|SetData (Variables|/Script/LidarPointCloudRuntime.LidarPointCloudComponent|GetPointCloud (Variables|/Game/MyRealisticMap/BP_PC.BP_PC_C|GetPC_Geo (Variables|Default|GetBP_PC_Ref))) (stale EventTick _lidarpointsout))
  (Variables|Default|SetScanCompleted true))

(event EventTick
  (params (DeltaSeconds :type Float%20%28single-precision%29))
  (if (Variables|Default|GetLidarTrigger)
    (bind _returnvalue (Actor|GetActorOfClass "/Game/MyRealisticMap/BP_PC.BP_PC_C"))
    (Variables|Default|SetBP_PC_Ref _returnvalue)
    (if (Variables|/Game/MyRealisticMap/BP_PC.BP_PC_C|GetCreate%20PC (Variables|Default|GetBP_PC_Ref))
      (if (Variables|Default|GetScanCompleted)
        (Variables|Default|SetScanCompleted false)
        (bind (_lidarpointsout _deptharrayout) (Class|LidarSensorSimulatorBPLibrary|LidarSensorAsyncScan2 (Variables|Default|GetPC_Points%20) (Variables|Default|GetSM_lidar) (delegate Custom|CustomEvent_1) true -15.0 15.0 (Variables|Default|GetChannel) 3.6e+02 (Variables|Default|GetResolution) (Variables|Default|GetDistance)))))))

(event EventBeginPlay
  (bind _returnvalue (Game|GetPlayerController 0))
  (Variables|/Script/Engine.PlayerController|SetbEnableClickEvents _returnvalue true)
  (Variables|/Script/Engine.PlayerController|SetbShowMouseCursor _returnvalue true))

(fn ConstructionScript)

(fn GetDepthmap)

(fn GetLocalPointCloud
  (bind _output_get (Variables|Default|Setray_point_location (Math|Vector|MakeVector (* (Variables|Default|GetRayDepth) (Math|Trig|Cos(Degrees) (Variables|Default|GetRayAngle))) (* (Variables|Default|GetRayDepth) (Math|Trig|Sin(Degrees) (Variables|Default|GetRayAngle))) 0.0)))
  (Utilities|Array|Add (Variables|Default|Getray_point_cloud) (Math|Transform|TransformLocation (Transformation|GetActorTransform) _output_get)))