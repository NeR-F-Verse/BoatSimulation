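; Simulated lidar sensor actor, apparently for a boat, with a GetDepthmap function that sends byte depth data over UDP.
; Play start enables mouse clicks, and clicking the lidar mesh prints the depthmap length.
; The scan code, vertically stacked fans of line traces filling depth and point-cloud arrays, is disconnected, so LidarLocationSetting does nothing.
; GetLocalPointCloud rebuilds a world point from ray depth and angle, but only disconnected code calls it.
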(event OnClicked(SM_lidar)
  (params (TouchedComponent :type Primitive%20Component%20Object%20Reference) (ButtonPressed :type Key%20Structure :default "None"))
  (Development|PrintString (Utilities|String|ToString(Integer) (Utilities|Array|Length (Variables|Default|GetDepthmap))) true false))

(event EventTick
  (params (DeltaSeconds :type Float%20%28single-precision%29)))

(event EventBeginPlay
  (bind _returnvalue (Game|GetPlayerController 0))
  (Variables|/Script/Engine.PlayerController|SetbEnableClickEvents _returnvalue true)
  (Variables|/Script/Engine.PlayerController|SetbShowMouseCursor _returnvalue true))

(fn ConstructionScript)

(fn LidarLocationSetting
  (params (boat_location :type Vector)))

(fn GetDepthmap
  (Class|UDPComponent|EmitBytes (Variables|Default|GetUDP) (Variables|Default|GetByte%20Depthmap)))

(fn GetLocalPointCloud
  (bind _output_get (Variables|Default|Setray_point_location (Math|Vector|MakeVector (* (Variables|Default|GetRayDepth) (Math|Trig|Cos(Degrees) (Variables|Default|GetRayAngle))) (* (Variables|Default|GetRayDepth) (Math|Trig|Sin(Degrees) (Variables|Default|GetRayAngle))) 0.0)))
  (Utilities|Array|Add (Variables|Default|Getray_point_cloud) (Math|Transform|TransformLocation (Transformation|GetActorTransform) _output_get)))