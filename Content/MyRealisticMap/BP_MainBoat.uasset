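; Player-controlled yacht that serves as a sensor simulation platform, streaming 360 lidar data over UDP.
; A timeline moves it along BP_SplinePath; pausing it allows scrubbing or force-based steering.
; BeginPlay packs sensor metadata and tags meshes and water with custom-depth stencil values per semantic class.
; A throttled Tick emits indexed point, depth and color packets with a periodic info header, and optionally prints a noisy GPS position.
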(event Custom|SceneCapture2img_Event
  ;[1 1 1] 좌표계 수정 부분
)

(event Custom|Move%20Object
  (bind _spline_ref (Variables|Default|GetSpline%20REF))
  (bind _spline (Variables|/Game/MyRealisticMap/BP_SplinePath.BP_SplinePath_C|GetSpline _spline_ref))
  ;[1 1 1] Move Object
  (Components|Timeline|SetPlayRate (Variables|Default|GetMove%20Object%20T) (/ 1.0 (Variables|Default|GetTime%20To%20Complete%20%28In%20Seconds%29)))
  (bind _move_track (Timeline|Move%20Object%20T Play)
    (:Update
      (Transformation|SetActorTransform (Math|Transform|MakeTransform (Spline|GetLocationatDistanceAlongSpline _spline (Math|Float|Lerp 0.0 (Spline|GetSplineLength (Variables|/Game/MyRealisticMap/BP_SplinePath.BP_SplinePath_C|GetSpline (Variables|Default|GetSpline%20REF))) _move_track) "World") (Math|Rotator|MakeRotator (.Roll (Math|Rotator|BreakRotator (Spline|GetRotationatDistanceAlongSpline _spline (Math|Float|Lerp 0.0 (Spline|GetSplineLength (Variables|/Game/MyRealisticMap/BP_SplinePath.BP_SplinePath_C|GetSpline (Variables|Default|GetSpline%20REF))) _move_track) "Local"))) (.Pitch (Math|Rotator|BreakRotator (Spline|GetRotationatDistanceAlongSpline _spline (Math|Float|Lerp 0.0 (Spline|GetSplineLength (Variables|/Game/MyRealisticMap/BP_SplinePath.BP_SplinePath_C|GetSpline (Variables|Default|GetSpline%20REF))) _move_track) "Local"))) (+ (.Yaw (Math|Rotator|BreakRotator (Spline|GetRotationatDistanceAlongSpline _spline (Math|Float|Lerp 0.0 (Spline|GetSplineLength (Variables|/Game/MyRealisticMap/BP_SplinePath.BP_SplinePath_C|GetSpline (Variables|Default|GetSpline%20REF))) _move_track) "Local"))) -9e+01)) "1.000000,1.000000,1.000000")))))

(event Custom|CustomEvent
  (for _array_element (Variables|Default|GetPackets)
    (bind _bytes (Class|SensorSimulatorBPLibrary|InttoBytes (Variables|Default|GetUDPCommunicationCount)))
    (bind _output_get (Variables|Default|Setpacket%20byte _bytes))
    (Utilities|Array|AppendArray _output_get (Utilities|Struct|BreakBytes _array_element))
    (Class|UDPComponent|EmitBytes (Variables|Components|GetUDP) (Variables|Default|Getpacket%20byte)))
  (bind _output_get_2 (Variables|Default|SetUDPCommunicationCount (+ (Variables|Default|GetUDPCommunicationCount) 1)))
  (Variables|Default|Setflag (== (Math|Integer|%(Integer) _output_get_2 100) 0)))

(event Custom|UDPSend_Event
  (Variables|Default|SetPacketIndex 0)
  (Variables|Default|SetIsBusy false)
  (Development|PrintString "Retry Connection!"))

(event EventBeginPlay
  (bind _sensorinfobytes (Variables|Default|GetSensorInfoBytes))
  (Utilities|FlowControl|Sequence
    (:then_0
      (bind _asbp_lidar_sensor_360 (Utilities|Casting|CastToBP_LidarSensor360 (Variables|/Script/Engine.ChildActorComponent|GetChildActor (Variables|Components|Getsensor360))))
      (for _array_element (Utilities|Array|MakeArray 1 (Variables|/Game/MyRealisticMap/BP_LidarSensor360.BP_LidarSensor360_C|GetLidarRes _asbp_lidar_sensor_360) (Variables|/Game/MyRealisticMap/BP_LidarSensor360.BP_LidarSensor360_C|GetLidarChannels _asbp_lidar_sensor_360) (Variables|/Game/MyRealisticMap/BP_LidarSensor360.BP_LidarSensor360_C|GetCaptureImageWidth _asbp_lidar_sensor_360) (Variables|/Game/MyRealisticMap/BP_LidarSensor360.BP_LidarSensor360_C|GetCaptureImageHeight _asbp_lidar_sensor_360))
        (bind _bytes (Class|SensorSimulatorBPLibrary|InttoBytes _array_element))
        (Utilities|Array|AppendArray _sensorinfobytes _bytes))
      (Utilities|Array|AppendArray _sensorinfobytes (Variables|/Game/MyRealisticMap/BP_LidarSensor360.BP_LidarSensor360_C|Getcamera_infos _asbp_lidar_sensor_360))
      (bind _bytes_2 (Class|SensorSimulatorBPLibrary|InttoBytes (Math|Conversions|ToInteger(Boolean) (Variables|/Game/MyRealisticMap/BP_LidarSensor360.BP_LidarSensor360_C|GetIsFisheye _asbp_lidar_sensor_360))))
      (Utilities|Array|AppendArray _sensorinfobytes _bytes_2)
      (Variables|Default|SetInitialized true))
    (:then_1
      (Actor|Tick|SetActorTickInterval 0.03))
    (:then_2
      (bind _enumvalue (|ForEachESemantic)
        (:LoopBody
          (CallFunction|SemanticSegmentation (Utilities|String|StringToName (Utilities|String|EnumtoString _enumvalue)) (Math|Conversions|ToInteger(Byte) _enumvalue)))))
    (:then_3
      ;[1 1 1] Move Object
      (Utilities|FlowControl|Delay 0.0)
      (bind _returnvalue (Actor|GetActorOfClass "/Game/MyRealisticMap/BP_SplinePath.BP_SplinePath_C"))
      (Variables|Default|SetSpline%20REF _returnvalue)
      (CallFunction|MoveObject))))

(event EventTick
  (params (DeltaSeconds :type Float%20%28single-precision%29))
  (bind _returnvalue (Math|Byte|MakeLiteralByte 255))
  (bind _sm_yacht (Variables|Components|GetSM_yacht))
  (bind _returnvalue_2 (Transformation|GetWorldLocation _sm_yacht))
  (Utilities|FlowControl|Sequence
    (:then_0
      ;[1 1 1] GPS 센서
      (if (Variables|Default|GetGPSTrigger)
        (Variables|Default|SetGPSlocation _returnvalue_2)
        (Development|PrintString (Utilities|String|ToString(Vector) (+ (* (Math|Conversions|ToVector(Float) (Class|KismetMathLibrary|FTruncVector (/ _returnvalue_2 "50.000000,50.000000,1.000000"))) "50.000000,50.000000,1.000000") (Math|Conversions|ToVector(Float) (Utilities|Struct|MakeIntVector (Math|Random|RandomInteger 50) (Math|Random|RandomInteger 50))))))))
    (:then_1
      (Utilities|FlowControl|Sequence
        (:then_0
          (if (Variables|Default|GetInitialized)
            (bind _asbp_lidar_sensor_360 (Utilities|Casting|CastToBP_LidarSensor360 (Variables|/Script/Engine.ChildActorComponent|GetChildActor (Variables|Default|GetSensor360))))
            (bind (_bytepackets _bytesinfo _bytespoints _bytescolormap _bytesdepthmap) (Class|SensorSimulatorBPLibrary|SensorOuttoBytes360 (Variables|/Game/MyRealisticMap/BP_LidarSensor360.BP_LidarSensor360_C|GetLidarSensorOut360 _asbp_lidar_sensor_360) (- (.BufferSize (Utilities|Struct|BreakUDPSettings (Variables|/Script/UDPWrapper.UDPComponent|GetSettings (Variables|Components|GetUDP)))) 8)))
            (bind _output_get (Variables|Default|SetpacketArray _bytepackets))
            (bind _output_get_2 (Variables|Default|SetPackets (Utilities|Struct|BreakTArrayBytes _bytepackets)))
            (Variables|Default|SetIndividualBytes (Utilities|Array|MakeArray _bytespoints _bytesdepthmap _bytescolormap))
            (Variables|Default|SetNumPackets (Utilities|Array|Length _output_get_2))
            (Utilities|FlowControl|Sequence
              (:then_0
                (Variables|Default|SetIsBusy true)
                (bind _output_get_3 (Variables|Default|SetInitialPacket (Utilities|Array|MakeArray _returnvalue _returnvalue _returnvalue _returnvalue))))
              (:then_1
                (if (> (Variables|Default|GetNumPackets) 0)
                  (bind _bytes (Class|SensorSimulatorBPLibrary|InttoBytes (Variables|Default|GetNumPackets)))
                  (Utilities|Array|AppendArray (Variables|Default|GetInitialPacket) _bytes)
                  (for _array_element (Variables|Default|GetIndividualBytes)
                    (bind _bytes_2 (Class|SensorSimulatorBPLibrary|InttoBytes _array_element))
                    (Utilities|Array|AppendArray _output_get_3 _bytes_2))
                  (if (Variables|Default|Getflag)
                    (Utilities|Array|AppendArray (Variables|Default|GetInitialPacket) (Variables|Default|GetSensorInfoBytes))
                    (Class|UDPComponent|EmitBytes (Variables|Components|GetUDP) (Variables|Default|GetInitialPacket))
                    (Variables|Default|Setflag false))
                  (else
                    (Variables|Default|SetIsBusy false)
                    (Development|PrintString "Preparing")))))))
        (:then_1
          (CallFunction|CustomEvent))))))

(event Input|AxisEvents|InputAxisMoveForward/Backward
  (params (AxisValue :type Float%20%28single-precision%29))
  ;[1 1 1] boat control
  (if (not (Audio|Components|Audio|IsPlaying (Variables|Default|GetMove%20Object%20T)))
    (Physics|AddForce (Variables|Components|GetSM_yacht) (* (* AxisValue 1e+03) (Transformation|GetActorRightVector)) "None" true)))

(event Input|AxisEvents|InputAxisMoveRight/Left
  (params (AxisValue :type Float%20%28single-precision%29))
  (bind _returnvalue (Transformation|GetActorRotation))
  (bind _returnvalue_2 (Transformation|GetActorRotation))
  (bind (_roll _pitch) (Math|Rotator|BreakRotator _returnvalue))
  (bind (_roll_2 _pitch_2) (Math|Rotator|BreakRotator _returnvalue_2))
  ;[1 1 1] boat control
  (if (not (Audio|Components|Audio|IsPlaying (Variables|Default|GetMove%20Object%20T)))
    (Physics|AddForce (Variables|Components|GetSM_yacht) (* (* AxisValue -1e+03) (Transformation|GetActorForwardVector)) "None" true)
    (if (!= (Input|AxisValues|GetMoveRight/Left) 0.0)
      (if (>= (Input|AxisValues|GetMoveForward/Backward) 0.0)
        (Transformation|SetActorRotation (Math|Rotator|MakeRotator _roll_2 _pitch_2 (.yaw (Math|Rotator|Lerp(Rotator) _returnvalue_2 (Math|Conversions|RotationFromXVector (Math|Vector|RotateVector (Transformation|GetVelocity) (Math|Rotator|MakeRotator 0.0 0.0 -9e+01))) 0.1 true))))
        (else
          (Transformation|SetActorRotation (Math|Rotator|MakeRotator _roll _pitch (.yaw (Math|Rotator|Lerp(Rotator) _returnvalue (Math|Conversions|RotationFromXVector (* (Math|Vector|RotateVector (Transformation|GetVelocity) (Math|Rotator|MakeRotator 0.0 0.0 -9e+01)) -1.0)) 0.1 true)))))))))

(event Input|KeyboardEvents|SpaceBar
  (params (Key :type Key%20Structure :default "None"))
  (bind _move_object_t (Variables|Default|GetMove%20Object%20T))
  (:Pressed
    (if (Audio|Components|Audio|IsPlaying (Variables|Default|GetMove%20Object%20T))
      (Audio|Components|Audio|Stop _move_object_t)
      (else
        (Audio|Components|Audio|Play _move_object_t)))))

(event Input|KeyboardEvents|O
  (params (Key :type Key%20Structure :default "None"))
  (bind _move_object_t (Variables|Default|GetMove%20Object%20T))
  (:Pressed
    (if (not (Audio|Components|Audio|IsPlaying (Variables|Default|GetMove%20Object%20T)))
      (Components|Timeline|SetNewTime _move_object_t (- (Components|Timeline|GetPlaybackPosition _move_object_t) 0.01)))))

(event Input|KeyboardEvents|P
  (params (Key :type Key%20Structure :default "None"))
  (bind _move_object_t (Variables|Default|GetMove%20Object%20T))
  (:Pressed
    (if (not (Audio|Components|Audio|IsPlaying (Variables|Default|GetMove%20Object%20T)))
      (Components|Timeline|SetNewTime _move_object_t (+ (Components|Timeline|GetPlaybackPosition _move_object_t) 0.01)))))

(fn ConstructionScript)

(fn SemanticSegmentation
  (params (Tag :type Name) (Value :type Integer))
  (if (== Tag "sea")
    (bind _returnvalue (Actor|GetActorOfClass "/Script/Water.WaterZone"))
    (Rendering|SetRenderCustomDepth (Variables|/Script/Water.WaterZone|GetWaterMesh _returnvalue) true)
    (Rendering|SetCustomDepthStencilValue (Variables|/Script/Water.WaterZone|GetWaterMesh _returnvalue) Value)
    (else
      (bind _outactors (Actor|GetAllActorswithTag Tag))
      (for _array_element _outactors
        (for _array_element_2 (Actor|GetComponentsbyTag _array_element "/Script/Engine.MeshComponent" Tag)
          (Rendering|SetRenderCustomDepth _array_element_2 true)
          (Rendering|SetCustomDepthStencilValue _array_element_2 Value))))))